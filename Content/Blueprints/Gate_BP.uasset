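; Gate actor that opens when its linked lever is activated, then removes itself from the level.
; Every Tick it gathers all Lever_BP actors and polls Activated on the one at array index LeverID, so the pairing depends on actor array order.
; Once that is true, it waits briefly, plays its ActorSequence component, and destroys itself after the sequence's duration.
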(event EventTick
  (params (DeltaSeconds :type Float%20%28single-precision%29))
  (bind _actorsequence (Variables|Default|GetActorSequence))
  (bind _sequenceplayer (Variables|/Script/ActorSequence.ActorSequenceComponent|GetSequencePlayer _actorsequence))
  (bind _outactors (Actor|GetAllActorsOfClass "/Game/Blueprints/Lever_BP.Lever_BP_C"))
  (if (Variables|/Script/Darkness3D.Lever|GetActivated (Utilities|Array|Get(acopy) _outactors (Variables|Default|GetLeverID)))
    (Utilities|FlowControl|Delay 1.0)
    (Sequencer|Player|Play _sequenceplayer :!class /Script/MovieScene.MovieSceneSequencePlayer)
    (Utilities|FlowControl|Delay (Class|TimeManagementBlueprintLibrary|ToSeconds(QualifiedFrameTime) (Media|MediaPlayer|GetDuration _sequenceplayer)))
    (Actor|DestroyActor)))

(fn ConstructionScript)