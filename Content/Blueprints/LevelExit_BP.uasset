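; LevelExit_BP is a level exit that opens and sends the game to the next level when an actor overlaps it.
; Tick plays its ActorSequence once, either when the cached player character has the key or right away in the Menu level.
; Any overlap, with no check on the actor or open state, clears all widgets, shows a loading screen and opens the next level by name after a one-second delay.
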(event EventBeginPlay
  (bind _returnvalue (Game|GetCurrentLevelName true))
  (if (Utilities|Enum|NotEqual(Enum) _returnvalue "Menu")
    (bind _asplayer_character_bp (Utilities|Casting|CastToPlayerCharacter_BP (Game|GetPlayerCharacter 0)))
    (Variables|Default|Setplayer _asplayer_character_bp)))

(event Collision|EventActorBeginOverlap
  (params (OtherActor :type Actor%20Object%20Reference))
  (Viewport|RemoveAllWidgets)
  (bind _returnvalue (UserInterface|CreateWidget "/Game/Blueprints/LoadingScreen.LoadingScreen_C" (Game|GetPlayerController 0)))
  (UserInterface|Viewport|AddtoViewport _returnvalue 0)
  (Utilities|FlowControl|Delay 1.0)
  (bind _returnvalue_2 (Class|LevelExit|GetNextLevelName))
  (Game|OpenLevel(byName) (Utilities|String|StringToName _returnvalue_2)))

(event EventTick
  (params (DeltaSeconds :type Float%20%28single-precision%29))
  (bind _returnvalue (Game|GetCurrentLevelName true))
  (if (Utilities|Enum|NotEqual(Enum) _returnvalue "Menu")
    (if (Variables|/Script/Darkness3D.PlayerCharacter|GethasKey (Variables|Default|Getplayer))
      (if (not (Variables|Default|GetisOpened))
        (Sequencer|Player|Play (Variables|/Script/ActorSequence.ActorSequenceComponent|GetSequencePlayer (Variables|Default|GetActorSequence)) :!class /Script/MovieScene.MovieSceneSequencePlayer)
        (Variables|Default|SetisOpened true)))
    (elif (not (Variables|Default|GetisOpened))
      (Sequencer|Player|Play (Variables|/Script/ActorSequence.ActorSequenceComponent|GetSequencePlayer (Variables|Default|GetActorSequence)) :!class /Script/MovieScene.MovieSceneSequencePlayer)
      (Variables|Default|SetisOpened true))))

(fn ConstructionScript)